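; BP_Cat is a player-controlled cat character that sits, stands up and walks along the world X axis.
; It adds the IMC_Cat Enhanced Input mapping on BeginPlay and routes stand, sit and walk actions through guard functions that check the CatState enum.
; Standing up and sitting down enter intermediate states, with SetStateStanding and SetStateSitting available to set the settled ones.
; Walking applies scaled-down movement input and returns to standing on release.
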(event Input|EnhancedActionEvents|EnhancedInputActionIA_Cat_SitDown
  (params (ActionValue :type Boolean) (ElapsedSeconds :type Float%20%28double-precision%29) (TriggeredSeconds :type Float%20%28double-precision%29) (InputAction :type Input%20Action%20Object%20Reference :default "/Game/Elke/Characters/Cat/Input/IA_Cat_SitDown.IA_Cat_SitDown"))
  (CallFunction|SitDown))

(event Input|EnhancedActionEvents|EnhancedInputActionIA_Cat_StandUp
  (params (ActionValue :type Boolean) (ElapsedSeconds :type Float%20%28double-precision%29) (TriggeredSeconds :type Float%20%28double-precision%29) (InputAction :type Input%20Action%20Object%20Reference :default "/Game/Elke/Characters/Cat/Input/IA_Cat_StandUp.IA_Cat_StandUp"))
  (CallFunction|StandUp))

(event Input|EnhancedActionEvents|EnhancedInputActionIA_Cat_Walk
  (params (ActionValue :type Float%20%28double-precision%29) (ElapsedSeconds :type Float%20%28double-precision%29) (TriggeredSeconds :type Float%20%28double-precision%29) (InputAction :type Input%20Action%20Object%20Reference :default "/Game/Elke/Characters/Cat/Input/IA_Cat_Walk.IA_Cat_Walk"))
  (:Triggered
    (if (CallFunction|CanWalk)
      (CallFunction|Walk ActionValue)))
  (:Completed
    (CallFunction|SetStateStanding)))

(event EventBeginPlay
  (bind _asplayer_controller (Utilities|Casting|CastToPlayerController (Pawn|GetController)))
  (Utilities|IsValid (PlayerController|LocalPlayerSubsystems|GetEnhancedInputLocalPlayerSubsystem _asplayer_controller)
    (:Is%20Valid
      (Input|AddMappingContext (PlayerController|LocalPlayerSubsystems|GetEnhancedInputLocalPlayerSubsystem _asplayer_controller) "/Game/Elke/Characters/Cat/Input/IMC_Cat.IMC_Cat" 0 "(bIgnoreAllPressedKeysUntilRelease=True,bForceImmediately=False,bNotifyUserSettings=False)"))))

(fn ConstructionScript)

(fn CanSitDown
  (return (Utilities|Enum|NotEqual(Enum) (Variables|Default|GetCat%20State) "NewEnumerator0")))

(fn CanStandUp
  (return (Utilities|Enum|Equal(Enum) (Variables|Default|GetCat%20State) "NewEnumerator0")))

(fn StandUp
  (if (CallFunction|CanStandUp)
    (Variables|Default|SetCat%20State "NewEnumerator2")))

(fn SetStateStanding
  (Variables|Default|SetCat%20State "NewEnumerator1"))

(fn SitDown
  (if (CallFunction|CanSitDown)
    (Variables|Default|SetCat%20State "NewEnumerator3")))

(fn Walk
  (params (Direction :type Float%20%28double-precision%29))
  (Variables|Default|SetCat%20State "NewEnumerator4")
  (Pawn|Input|AddMovementInput "1.000000,0.000000,0.000000" (* Direction 0.05) false))

(fn CanWalk
  (bind _cat_state (Variables|Default|GetCat%20State))
  (return (or (Utilities|Enum|Equal(Enum) _cat_state "NewEnumerator1") (Utilities|Enum|Equal(Enum) _cat_state "NewEnumerator4"))))

(fn SetStateSitting
  (Variables|Default|SetCat%20State "NewEnumerator0"))